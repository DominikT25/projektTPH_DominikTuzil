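; Launch pad variant that throws the overlapping character upward, built as a child of a parent launch pad Blueprint.
; It extends OnLaunch by running the parent logic, then calling LaunchCharacter on the inherited OverlappingCharacter if valid.
; LaunchVelocity replaces the character's Z velocity, while the unscaled forward X and Y are added to existing horizontal velocity, preserving momentum.
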(event `self.OnLaunch`
  (`parent.OnLaunch`)
  (bind _overlappingcharacter (`self.OverlappingCharacter`)
    (:`then`
      (bind (_returnvalue_x _returnvalue_y) (`KismetMathLibrary.BreakVector` (`self.GetActorForwardVector` _overlappingcharacter)))
      (`Character.LaunchCharacter` (`self.OverlappingCharacter`) (`KismetMathLibrary.MakeVector` _returnvalue_x _returnvalue_y (`self.LaunchVelocity`)) false true))
    (:`else`)))

(fn `UserConstructionScript`
  (`parent.UserConstructionScript`))