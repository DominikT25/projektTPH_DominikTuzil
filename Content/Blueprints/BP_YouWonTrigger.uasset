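; BP_YouWonTrigger is a trigger actor that ends the game when an actor tagged Player overlaps its collision.
; On overlap it shows the WB_YouWon widget, sets the game instance's last checkpoint to a hard-coded position and saves to a named slot.
; After a short delay it reopens ThirdPersonMap and calls the game instance's reset function on that same slot.
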(event `self.Collision.OnComponentBeginOverlap`
  (params (OverlappedComponent :type "PrimitiveComponent Object Reference") (OtherActor :type "Actor Object Reference") (OtherComp :type "PrimitiveComponent Object Reference") (OtherBodyIndex :type Integer) (bFromSweep :type Boolean) (SweepResult :type "HitResult Structure (by ref)"))
  (if (`self.ActorHasTag` OtherActor "Player")
    (bind _returnvalue (`|CreateWidget` "/Game/Blueprints/WB_YouWon.WB_YouWon_C"))
    (`UserWidget.AddToViewport` _returnvalue 0)
    (bind _asbp_game_instance (cast `/Game/Blueprints/BP_GameInstance` (`GameplayStatics.GetGameInstance`)))
    (set `/Game/Blueprints/BP_GameInstance.lastCheckpointVector` (-1260.0 350.0 101.986) _asbp_game_instance)
    (`/Game/Blueprints/BP_GameInstance.fSaveGame` _asbp_game_instance "Slot1")
    (`KismetSystemLibrary.Delay` 5.0)
    (`GameplayStatics.OpenLevel` "ThirdPersonMap")
    (`/Game/Blueprints/BP_GameInstance.fResetGame` _asbp_game_instance "Slot1")))

(fn `UserConstructionScript`)