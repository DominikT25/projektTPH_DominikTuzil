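; BP_Moving_Key_Forward_Backward is a moving hazard that applies BaseDamage to any actor that begins overlapping its Box.
; On BeginPlay it stores its starting location, then each Tick shifts an offset by Speed scaled by delta time, reversing direction at zero and MaxOffset.
; The offset is added to the starting world Y, so the actor ping-pongs along that axis at constant speed without sweeping or easing.
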(event `self.Box.OnComponentBeginOverlap`
  (params (OverlappedComponent :type "PrimitiveComponent Object Reference") (OtherActor :type "Actor Object Reference") (OtherComp :type "PrimitiveComponent Object Reference") (OtherBodyIndex :type Integer) (bFromSweep :type Boolean) (SweepResult :type "HitResult Structure (by ref)"))
  (`GameplayStatics.ApplyDamage` OtherActor (`self.Base Damage`)))

(event `self.ReceiveBeginPlay`
  (set `self.defaultLocation` (`self.K2_GetActorLocation`))
  (set `self.offset` 0.0)
  (set `self.bGoingRight` true))

(event `self.ReceiveTick`
  (params (DeltaSeconds :type "Float (single-precision)"))
  (bind (_defaultlocation_x _defaultlocation_y _defaultlocation_z) (`KismetMathLibrary.BreakVector` (`self.defaultLocation`)))
  (set `self.Step` (* DeltaSeconds (`self.Speed`)))
  (if (`self.bGoingRight`)
    (set `self.offset` (+ (`self.offset`) (`self.Step`)))
    (if (>= (`self.offset`) (`self.maxOffset`))
      (set `self.offset` (`self.maxOffset`))
      (set `self.bGoingRight` false))
    (else
      (set `self.offset` (- (`self.offset`) (`self.Step`)))
      (if (<= (`self.offset`) 0.0)
        (set `self.offset` 0.0)
        (set `self.bGoingRight` true))))
  (`self.K2_SetActorLocation` (`KismetMathLibrary.MakeVector` _defaultlocation_x (+ _defaultlocation_y (`self.offset`)) _defaultlocation_z)))

(fn `UserConstructionScript`)