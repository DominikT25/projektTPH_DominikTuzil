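; Pickup actor that gives the player a speed and jump boost on contact.
; When an actor tagged Player that implements BPI_PowerUp overlaps its collision, it sends SpeedBoostMessage with its Speed and Jump values.
; It then plays a camera shutter sound at its location and destroys itself, leaving the boost itself to the receiver.
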(event `self.Collision.OnComponentBeginOverlap`
  (params (OverlappedComponent :type "PrimitiveComponent Object Reference") (OtherActor :type "Actor Object Reference") (OtherComp :type "PrimitiveComponent Object Reference") (OtherBodyIndex :type Integer) (bFromSweep :type Boolean) (SweepResult :type "HitResult Structure (by ref)"))
  (if (`self.ActorHasTag` OtherActor "Player")
    (if (`KismetSystemLibrary.DoesImplementInterface` OtherActor "/Game/Blueprints/BPI_PowerUp.BPI_PowerUp_C")
      (message `/Game/Blueprints/BPI_PowerUp.Speed Boost` OtherActor (`self.Speed`) (`self.Jump`))
      (`GameplayStatics.PlaySoundAtLocation` "/Engine/VREditor/Sounds/UI/Camera_Shutter.Camera_Shutter" (`self.K2_GetActorLocation`) (struct) 0.8 1.0 0.0 null null null null)
      (`self.K2_DestroyActor`))))

(fn `UserConstructionScript`
  (`parent.UserConstructionScript`))