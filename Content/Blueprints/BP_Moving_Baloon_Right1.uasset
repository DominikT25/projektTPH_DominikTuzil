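; BP_Moving_Baloon_Right1 is a balloon actor that oscillates along the world X axis from its starting location.
; Each Tick moves an Offset by Speed scaled by delta time, reversing direction at MaxOffset and at zero.
; The location is rebuilt from the position saved at BeginPlay plus that Offset.
; When FlyUp is set, the same Offset is also added to Z, making the path a back-and-forth diagonal.
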(event `self.ReceiveBeginPlay`
  (set `self.defaultLocation` (`self.K2_GetActorLocation`))
  (set `self.offset` 0.0)
  (set `self.bGoingRight` true))

(event `self.ReceiveTick`
  (params (DeltaSeconds :type "Float (single-precision)"))
  (bind (_returnvalue_x _returnvalue_y _returnvalue_z) (`KismetMathLibrary.BreakVector` (`self.K2_GetActorLocation`)))
  (bind (_defaultlocation_x _defaultlocation_y _defaultlocation_z) (`KismetMathLibrary.BreakVector` (`self.defaultLocation`)))
  (set `self.Step` (* DeltaSeconds (`self.Speed`)))
  (if (`self.bGoingRight`)
    (set `self.offset` (+ (`self.offset`) (`self.Step`)))
    (if (>= (`self.offset`) (`self.maxOffset`))
      (set `self.offset` (`self.maxOffset`))
      (set `self.bGoingRight` false))
    (else
      (set `self.offset` (- (`self.offset`) (`self.Step`)))
      (if (<= (`self.offset`) 0.0)
        (set `self.offset` 0.0)
        (set `self.bGoingRight` true))))
  (`self.K2_SetActorLocation` (`KismetMathLibrary.MakeVector` (+ _defaultlocation_x (`self.offset`)) _defaultlocation_y _defaultlocation_z))
  (if (`self.flyUp`)
    (bind _output_get (set `self.zLocation` (+ _returnvalue_z (`self.offset`))))
    (`self.K2_SetActorLocation` (`KismetMathLibrary.MakeVector` _returnvalue_x _returnvalue_y _output_get))))

(fn `UserConstructionScript`)