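; BP_Skul_MovingUp is an actor that oscillates vertically between its spawn height and a maximum offset above it.
; BeginPlay caches the starting location and sets it moving upward.
; Tick advances a Z offset by Speed scaled by delta time, clamps it at either limit to flip direction, and sets the actor location from the cached position, giving frame-rate-independent linear ping-pong motion.
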(event `self.ReceiveBeginPlay`
  (set `self.defaultLocation` (`self.K2_GetActorLocation`))
  (set `self.zOffset` 0.0)
  (set `self.bGoingUp` true))

(event `self.ReceiveTick`
  (params (DeltaSeconds :type "Float (single-precision)"))
  (bind (_defaultlocation_x _defaultlocation_y _defaultlocation_z) (`KismetMathLibrary.BreakVector` (`self.defaultLocation`)))
  (set `self.Step` (* DeltaSeconds (`self.Speed`)))
  (if (`self.bGoingUp`)
    (set `self.zOffset` (+ (`self.zOffset`) (`self.Step`)))
    (if (>= (`self.zOffset`) (`self.maxOffset`))
      (set `self.zOffset` (`self.maxOffset`))
      (set `self.bGoingUp` false))
    (else
      (set `self.zOffset` (- (`self.zOffset`) (`self.Step`)))
      (if (<= (`self.zOffset`) 0.0)
        (set `self.zOffset` 0.0)
        (set `self.bGoingUp` true))))
  (`self.K2_SetActorLocation` (`KismetMathLibrary.MakeVector` _defaultlocation_x _defaultlocation_y (+ _defaultlocation_z (`self.zOffset`)))))

(fn `UserConstructionScript`)