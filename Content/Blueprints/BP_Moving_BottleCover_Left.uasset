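; BP_Moving_BottleCover_Left is a moving actor, named as a bottle cover, that slides back and forth along the world X axis.
; BeginPlay caches the start location, and Tick advances an offset by Speed scaled by delta time, clamping and reversing at zero and MaxOffset.
; Each frame it sets the location to the start minus the offset, so it first moves toward negative X, then returns.
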(event `self.ReceiveBeginPlay`
  (set `self.defaultLocation` (`self.K2_GetActorLocation`))
  (set `self.xOffset` 0.0)
  (set `self.bGoingLeft` true))

(event `self.ReceiveTick`
  (params (DeltaSeconds :type "Float (single-precision)"))
  (bind (_defaultlocation_x _defaultlocation_y _defaultlocation_z) (`KismetMathLibrary.BreakVector` (`self.defaultLocation`)))
  (set `self.Step` (* DeltaSeconds (`self.Speed`)))
  (if (`self.bGoingLeft`)
    (set `self.xOffset` (+ (`self.xOffset`) (`self.Step`)))
    (if (>= (`self.xOffset`) (`self.maxOffset`))
      (set `self.xOffset` (`self.maxOffset`))
      (set `self.bGoingLeft` false))
    (else
      (set `self.xOffset` (- (`self.xOffset`) (`self.Step`)))
      (if (<= (`self.xOffset`) 0.0)
        (set `self.xOffset` 0.0)
        (set `self.bGoingLeft` true))))
  (`self.K2_SetActorLocation` (`KismetMathLibrary.MakeVector` (- _defaultlocation_x (`self.xOffset`)) _defaultlocation_y _defaultlocation_z)))

(fn `UserConstructionScript`)