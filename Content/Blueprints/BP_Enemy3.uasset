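; BP_Enemy3 is a patrolling enemy that walks forward constantly, attacks what it runs into and can be killed by a stomp.
; A downward sphere trace ahead detects missing floor and, gated by a DoOnce, turns it 180 degrees.
; While alive, a second sphere trace plays a crowbar attack animation and damages the hit actor.
; Player feet overlapping DamageCollision ragdoll the enemy, disable its movement and launch the player upward.
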(event `self.ReceiveTick`
  (params (DeltaSeconds :type "Float (single-precision)"))
  (bind _charactermovement (`self.CharacterMovement`))
  (`|ExecutionSequence`
    (:`then_0`
      (bind _floor_detected (`self.LineTrace for Obstacle`))
      (if _floor_detected
        (goto _label :!via `Reset`)
        (else
          (`/Engine/EditorBlueprintResources/StandardMacros.DoOnce` false :!label _label
            (:`Completed`
              (`/Engine/EditorBlueprintResources/StandardMacros.FlipFlop`
                (:`A`
                  (`MovementComponent.StopMovementImmediately` _charactermovement)
                  (`self.K2_AddActorWorldRotation` (struct :`Yaw` 180.0)))
                (:`B`
                  (`MovementComponent.StopMovementImmediately` _charactermovement)
                  (`self.K2_AddActorWorldRotation` (struct :`Yaw` 180.0)))))))))
    (:`then_1`
      (`self.Move Forward`))
    (:`then_2`
      (if (not (`self.isDead`))
        (`self.LineTrace for Damage`)))))

(event `Move Forward`
  (`self.AddMovementInput` (`self.GetActorForwardVector`)))

(event `self.Damage Collision.OnComponentBeginOverlap`
  (params (OverlappedComponent :type "PrimitiveComponent Object Reference") (OtherActor :type "Actor Object Reference") (OtherComp :type "PrimitiveComponent Object Reference") (OtherBodyIndex :type Integer) (bFromSweep :type Boolean) (SweepResult :type "HitResult Structure (by ref)"))
  (if (and (`self.ActorHasTag` OtherActor "Player") (`ActorComponent.ComponentHasTag` OtherComp "Player Feet"))
    (`PrimitiveComponent.SetSimulatePhysics` (`self.Mesh`) true)
    (`CharacterMovementComponent.DisableMovement` (`self.CharacterMovement`))
    (`ActorComponent.K2_DestroyComponent` (`self.Box`))
    (`PrimitiveComponent.SetCollisionResponseToChannel` (`self.CapsuleComponent`) "ECC_Pawn" "ECR_Ignore")
    (`PrimitiveComponent.SetCollisionResponseToChannel` (`self.Mesh`) "ECC_Camera" "ECR_Ignore")
    (`PrimitiveComponent.SetCollisionResponseToChannel` (`self.CapsuleComponent`) "ECC_Camera" "ECR_Ignore")
    (set `self.isDead` true)
    (bind _asbp_third_person_character (cast `/Game/ThirdPerson/Blueprints/BP_ThirdPersonCharacter` OtherActor))
    (`self.LaunchCharacter` _asbp_third_person_character (* (`KismetMathLibrary.GetUpVector` (`self.K2_GetActorRotation` _asbp_third_person_character)) 500.0) false false)
    (`PrimitiveComponent.SetCollisionEnabled` (`self.Damage Collision`) "NoCollision")))

(fn `LineTrace for Damage`
  (bind _attack_damage_pos (`self.Attack Damage Pos`))
  (bind _returnvalue (`SceneComponent.K2_GetComponentLocation` _attack_damage_pos))
  (bind (_outhit _returnvalue_2) (`KismetSystemLibrary.SphereTraceSingle` :`Start` _returnvalue :`End` (+ _returnvalue (* (`SceneComponent.K2_GetComponentRotation` _attack_damage_pos) 35.0)) :`Radius` 20.0 :`TraceChannel` "TraceTypeQuery1" :`DrawTime` 1.0))
  (if _returnvalue_2
    (`SkeletalMeshComponent.PlayAnimation` (`self.Mesh`) "/Game/Interaction/Animations/CloseCombat/Takedown/Crowbar/A_TD_Crowbar_Attacker_01.A_TD_Crowbar_Attacker_01" false)
    (`GameplayStatics.ApplyDamage` (`.HitActor` (`GameplayStatics.BreakHitResult` _outhit)) 100.0)))

(fn `LineTrace for Obstacle`
  (returns (`Floor Detected` :type Boolean))
  (bind _returnvalue (`SceneComponent.K2_GetComponentLocation` (`self.LineTrace Floor Pos`)))
  (bind (_outhit _returnvalue_2) (`KismetSystemLibrary.SphereTraceSingle` :`Start` _returnvalue :`End` (+ _returnvalue (* (`KismetMathLibrary.GetUpVector` (`self.K2_GetActorRotation`)) -100.0)) :`Radius` 15.0 :`TraceChannel` "TraceTypeQuery1" :`DrawTime` 0.1))
  (return _returnvalue_2))

(fn `UserConstructionScript`)